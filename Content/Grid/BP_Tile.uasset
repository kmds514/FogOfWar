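; BP_Tile is a grid tile actor with a sphere, a plane and a fog state.
; The construction script sizes the sphere from SphereRadius and scales the plane in X and Y to sit just inside its diameter.
; The ToGrey event switches FogState after a short delay.
; BeginPlay sets a timer by name for DrawDebugTile, which is an empty function.
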(event `self.ReceiveBeginPlay`
  (`KismetSystemLibrary.K2_SetTimer` null "DrawDebugTile"))

(event `ToGrey`
  (`KismetSystemLibrary.Delay` 0.5)
  (set `self.FogState` "NewEnumerator2"))

(fn `DrawDebugTile`)

(fn `UserConstructionScript`
  (bind _returnvalue (* (`self.SphereRadius`) 0.019))
  (`SphereComponent.SetSphereRadius` (`self.Sphere`) (`self.SphereRadius`) true)
  (`SceneComponent.SetWorldScale3D` (`self.Plane`) (`KismetMathLibrary.MakeVector` _returnvalue _returnvalue 1.0)))