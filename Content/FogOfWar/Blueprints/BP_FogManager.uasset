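; Fog of war manager that renders fog through a post-process material and on the player's minimap.
; BeginPlay creates both dynamic materials, passes TopDownGrid bounds to the post-process one, creates a grid-resolution render target and starts a minimap update timer.
; Each Tick draws the current fog texture into that target with delta-time-scaled alpha, blending changes over time.
; The minimap update feeds the fog texture directly to its material, without that blending.
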(event `self.ReceiveBeginPlay`
  (bind _returnvalue (`TopDownGrid.GetGridResolution` (`self.TopDownGrid`)))
  ;[1 0 0.031] BeginPlay
  (`|ExecutionSequence`
    (:`then_0`
      ;[1 1 1] 포스트 프로세스 머티리얼 생성 및 등록
      (bind _returnvalue_2 (`KismetMaterialLibrary.CreateDynamicMaterialInstance` "/Game/FogOfWar/Materials/PP_FogOfWar.PP_FogOfWar"))
      (set `self.FogOfWarDMI` _returnvalue_2)
      (set `PostProcessComponent.bUnbound` false (`self.PostProcess`))
      (set `PostProcessComponent.Settings` (make `PostProcessSettings` :`WeightedBlendables` (make `WeightedBlendables` (`|MakeArray` (make `WeightedBlendable` 1.0 (`self.FogOfWarDMI`))))) (`self.PostProcess`)))
    (:`then_1`
      ;[1 1 1] 미니맵 머티리얼 생성
      (bind _returnvalue_3 (`KismetMaterialLibrary.CreateDynamicMaterialInstance` "/Game/FogOfWar/Materials/M_FogMinimap.M_FogMinimap"))
      (set `self.FogMiniMapDMI` _returnvalue_3))
    (:`then_2`
      ;[1 1 1] 포스트 프로세스 머티리얼 파라미터 설정
      (`KismetSystemLibrary.Delay` 0.2)
      (`/Engine/EditorBlueprintResources/StandardMacros.IsValid` (`self.TopDownGrid`)
        (:`Is Valid`
          (`MaterialInstanceDynamic.SetScalarParameterValue` (`self.FogOfWarDMI`) "GridExtent" (`KismetMathLibrary.Conv_IntToDouble` (`TopDownGrid.GetGridVolumeExtentXY` (`self.TopDownGrid`))))
          (`MaterialInstanceDynamic.SetScalarParameterValue` (`self.FogOfWarDMI`) "BlurDistance" (`self.FogBlurDistance`))
          (`MaterialInstanceDynamic.SetVectorParameterValue` (`self.FogOfWarDMI`) "GridLocation" (`KismetMathLibrary.Conv_VectorToLinearColor` (`self.K2_GetActorLocation` (`self.TopDownGrid`)))))))
    (:`then_3`
      ;[1 1 1] 캔버스 생성
      (`KismetSystemLibrary.Delay` 1.0)
      (bind _returnvalue_4 (`CanvasRenderTarget2D.CreateCanvasRenderTarget2D` "/Script/Engine.CanvasRenderTarget2D" _returnvalue _returnvalue))
      (set `self.FogCanvasRT` _returnvalue_4)
      (set `TextureRenderTarget2D.AddressX` "TA_Clamp" (`self.FogCanvasRT`))
      (set `TextureRenderTarget2D.AddressY` "TA_Clamp" (`self.FogCanvasRT`))
      (`KismetRenderingLibrary.ClearRenderTarget2D` (`self.FogCanvasRT`))
      (`MaterialInstanceDynamic.SetTextureParameterValue` (`self.FogOfWarDMI`) "FogTexture" (`self.FogCanvasRT`)))
    (:`then_4`
      ;[1 1 1] 미니맵 업데이트 타이머 설정
      (`KismetSystemLibrary.K2_SetTimerDelegate` (`|CreateDelegate` :!event `UpdateMinimapDMI`) (/ 1.0 (`KismetMathLibrary.Conv_ByteToDouble` (`self.FogUpdateInterval`))) true))))

(event `UpdateMinimapDMI`
  ;[1 1 1] 미니맵 업데이트
  (`MaterialInstanceDynamic.SetTextureParameterValue` (`self.FogMiniMapDMI`) "FogTexture" (`self.GetFogTexture`))
  (`Image.SetBrushFromMaterial` (`/Game/UI/Blueprints/WBP_Minimap.MinimapImage` (`/Game/TopDown/Blueprints/BP_TopDownPlayerController.MiniMapWBP` (cast `/Game/TopDown/Blueprints/BP_TopDownPlayerController` (`GameplayStatics.GetPlayerController` 0) :!pure true))) (`self.FogMiniMapDMI`)))

(event `DrawFog`
  ;[1 1 1] 포스트 프로세스에서 사용할 안개 텍스처 업데이트
  (`/Engine/EditorBlueprintResources/StandardMacros.IsValid` (`self.FogCanvasRT`)
    (:`Is Valid`
      (bind (_canvas _size _context) (`KismetRenderingLibrary.BeginDrawCanvasToRenderTarget` (`self.FogCanvasRT`)))
      (`Canvas.K2_DrawTexture` _canvas (`self.GetFogTexture`) (0.0 0.0) _size (0.0 0.0) (1.0 1.0) (`KismetMathLibrary.MakeColor` 1.0 1.0 1.0 (* (`KismetMathLibrary.Conv_ByteToInt` (`self.FogInterpSpeed`)) (`GameplayStatics.GetWorldDeltaSeconds`))) "BLEND_Translucent" 0.0 (0.5 0.5))
      (`KismetRenderingLibrary.EndDrawCanvasToRenderTarget` _context))))

(event `self.ReceiveTick`
  (params (DeltaSeconds :type "Float (single-precision)"))
  ;[1 0 0] Tick
  (`|ExecutionSequence`
    (:`then_0`
      (`self.DrawFog`))))

(fn `UserConstructionScript`)