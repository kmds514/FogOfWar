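; Lobby game state that tracks connected players and a game start countdown for the lobby UI.
; Add and remove functions maintain the connected controller list and set the player count from its length.
; RepNotifies on the count and countdown tell the local lobby player controller to update its display.
; The countdown notify uses a controller reference cached at BeginPlay, while the count notify casts afresh each time.
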(event `self.ReceiveBeginPlay`
  (bind _asbp_lobby_player_controller (cast `/Game/Core/Blueprints/BP_LobbyPlayerController` (`GameplayStatics.GetPlayerController` 0)))
  (set `self.LobbyPlayerController` _asbp_lobby_player_controller))

(fn `AddPlayer`
  (params (PlayerController :type "PlayerController Object Reference (by ref)"))
  (bind _connectedplayers (`self.ConnectedPlayers`))
  (`KismetArrayLibrary.Array_Add` _connectedplayers PlayerController)
  (set `self.NumOfPlayers` (`KismetArrayLibrary.Array_Length` _connectedplayers)))

(fn `OnRep_GameStartCountdown`
  (`/Engine/EditorBlueprintResources/StandardMacros.IsValid` (`self.LobbyPlayerController`)
    (:`Is Valid`
      (`/Game/Core/Blueprints/BP_LobbyPlayerController.UpdateCountdown` (`self.LobbyPlayerController`)))))

(fn `OnRep_NumOfPlayers`
  (bind _asbp_lobby_player_controller (cast `/Game/Core/Blueprints/BP_LobbyPlayerController` (`GameplayStatics.GetPlayerController` 0))
    (:`then`
      (`/Game/Core/Blueprints/BP_LobbyPlayerController.UpdateNumOfPlayers` _asbp_lobby_player_controller))
    (:`CastFailed`
      (`KismetSystemLibrary.PrintString` "Failed to cast LobbyPC"))))

(fn `RemovePlayer`
  (params (PlayerController :type "Controller Object Reference (by ref)"))
  (bind _connectedplayers (`self.ConnectedPlayers`))
  (`KismetArrayLibrary.Array_RemoveItem` _connectedplayers PlayerController)
  (set `self.NumOfPlayers` (`KismetArrayLibrary.Array_Length` _connectedplayers)))

(fn `UserConstructionScript`)