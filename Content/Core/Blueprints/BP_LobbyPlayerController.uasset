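; Player controller for the multiplayer lobby, linking each client's lobby UI to BP_LobbyGameMode.
; On init it saves name, team ID and an index-based team color to BP_GameInstance, then sends that info to the server.
; Client events drive the lobby menu, player list, map settings and loading screen, while server-received chat is relayed to every lobby controller.
; It destroys the session on EndPlay.
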(event `self.ReceiveEndPlay`
  (params (EndPlayReason :type "EEndPlayReason Enum" :default "Destroyed"))
  (`DestroySessionCallbackProxy.DestroySession` self))

(event `Client_InitializeLobbyPC`
  (params (PlayerIndex :type Integer))
  ;[1 1 1] 플레이어 컨트롤러 초기화
  (bind _asbp_game_instance (cast `/Game/Core/Blueprints/BP_GameInstance` (`GameplayStatics.GetGameInstance`)))
  (`TopDownGameInstance.SetPlayerInfo` _asbp_game_instance (`self.GetUserName`) PlayerIndex (select `int` PlayerIndex :`0` (struct :`R` 0.7 :`A` 1.0) :`1` (struct :`G` 0.04 :`B` 0.8 :`A` 1.0) :`2` (struct :`G` 0.6 :`B` 0.6 :`A` 1.0) :`3` (struct :`R` 0.15 :`B` 0.3 :`A` 1.0) :!type "LinearColor Structure"))
  (bind _output_get (set `self.PlayerInfo` (`TopDownGameInstance.PlayerInfo` _asbp_game_instance)))
  (`self.Server_UpdatePlayerInfo` _output_get))

(event `Server_UpdatePlayerInfo`
  (params (PlayerInfo :type "PlayerInfo Structure"))
  ;[1 1 1] 서버에게 PlayerInfo를 업데이트하라고 호출
  (set `self.PlayerInfo` PlayerInfo)
  (bind _asbp_lobby_game_mode (cast `/Game/Core/Blueprints/BP_LobbyGameMode` (`GameplayStatics.GetGameMode`)))
  (`/Game/Core/Blueprints/BP_LobbyGameMode.Server_UpdatePlayerInfo` _asbp_lobby_game_mode))

(event `Client_CreateLobbyMenu`
  (params (ServerName :type Text))
  ;[1 1 1] LobbyMenu 위젯을 만들고 화면에 출력
  (bind _returnvalue (`|CreateWidget` "/Game/UI/Blueprints/WBP_LobbyMenu.WBP_LobbyMenu_C" null ServerName))
  (bind _output_get (set `self.LobbyMenuWBP` _returnvalue))
  (`UserWidget.AddToViewport` _output_get 0)
  (`WidgetBlueprintLibrary.SetInputMode_GameAndUIEx` self (`self.LobbyMenuWBP`) "DoNotLock" false))

(event `Client_AddPlayerInfo`
  (params (ConnectedPlayerInfo :type "Array of PlayerInfo Structure"))
  ;[1 1 1] PlayerInfo 업데이트
  (set `self.ConnectedPlayers` ConnectedPlayerInfo)
  (`/Engine/EditorBlueprintResources/StandardMacros.IsValid` (`self.LobbyMenuWBP`)
    (:`Is Valid`
      (`/Game/UI/Blueprints/WBP_LobbyMenu.ClearPlayerList` (`self.LobbyMenuWBP`))
      (for (_array_element _array_index) (`self.ConnectedPlayers`)
        (`/Game/UI/Blueprints/WBP_LobbyMenu.Client_UpdatePlayerWindow` (`self.LobbyMenuWBP`) _array_element _array_index)))))

(event `Client_UpdateLobbySettings`
  (params (MapImage :type "Texture2D Object Reference") (MapName :type Text))
  (bind _lobbymenuwbp (`self.LobbyMenuWBP`))
  ;[1 1 1] 로비 설정 업데이트
  (set `/Game/UI/Blueprints/WBP_LobbyMenu.MapImage` MapImage _lobbymenuwbp)
  (set `/Game/UI/Blueprints/WBP_LobbyMenu.MapName` MapName _lobbymenuwbp))

(event `Client_ShowLoadingScreen`
  ;[1 1 1] 로비 메뉴 화면을 없애고 로딩 화면으로 전환
  (`Widget.RemoveFromParent` (`self.LobbyMenuWBP`))
  (bind _returnvalue (`|CreateWidget` "/Game/UI/Blueprints/WBP_LoadingScreen.WBP_LoadingScreen_C" self))
  (`UserWidget.AddToViewport` _returnvalue 0))

(event `Server_SendChatMessage`
  (params (Message :type Text))
  ;[1 1 1] 받은 메시지를 클라이언트에 전달
  (set `self.SenderMessage` Message)
  (set `self.SenderName` (`.Name` (break `PlayerInfo` (`self.PlayerInfo`))))
  (bind _asbp_lobby_game_mode (cast `/Game/Core/Blueprints/BP_LobbyGameMode` (`GameplayStatics.GetGameMode`)))
  (for _array_element (`/Game/Core/Blueprints/BP_LobbyGameMode.AllPlayerControllers` _asbp_lobby_game_mode)
    (bind _asbp_lobby_player_controller (cast `/Game/Core/Blueprints/BP_LobbyPlayerController` _array_element))
    (`self.Client_UpdateChatMessage` _asbp_lobby_player_controller (`self.SenderName`) (`self.SenderMessage`))))

(event `Client_UpdateChatMessage`
  (params (Sneder :type Text) (Message :type Text))
  ;[1 1 1] 클라이언트에서 채팅 출력
  (`/Game/UI/Blueprints/WBP_LobbyMenu.Client_UpdateChatWindow` (`self.LobbyMenuWBP`) Sneder Message))

(fn `GetUserName`
  (returns (Name :type Text))
  (bind _asbp_game_instance (cast `/Game/Core/Blueprints/BP_GameInstance` (`GameplayStatics.GetGameInstance`))
    (:`then`
      (return (`TopDownGameInstance.GetUserName` _asbp_game_instance)))
    (:`CastFailed`
      (`KismetSystemLibrary.PrintString` "Failed to cast GameInstanceBP" true true (struct :`G` 0.66 :`B` 1.0 :`A` 1.0) 10.0))))

(fn `UserConstructionScript`)