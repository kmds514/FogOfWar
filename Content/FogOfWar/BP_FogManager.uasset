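; Fog of war manager that displays a fog texture through a post-process material and on the player's minimap.
; On BeginPlay it puts a dynamic material on its bounded post-process component, then after a short delay scales it to the TopDownGrid extent and starts a looping timer based on FogUpdateInterval.
; The update event pushes FogTexture to the material and minimap image; the texture itself is generated outside these graphs.
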(event `self.ReceiveBeginPlay`
  (`|ExecutionSequence`
    (:`then_0`
      (bind _returnvalue (`KismetMaterialLibrary.CreateDynamicMaterialInstance` "/Game/FogOfWar/PP_FogOfWar.PP_FogOfWar"))
      (set `self.PostProcessDMI` _returnvalue)
      (set `PostProcessComponent.bUnbound` false (`self.PostProcess`))
      (set `PostProcessComponent.Settings` (make `PostProcessSettings` :`WeightedBlendables` (make `WeightedBlendables` (`|MakeArray` (make `WeightedBlendable` 1.0 (`self.PostProcessDMI`))))) (`self.PostProcess`)))
    (:`then_1`
      (`KismetSystemLibrary.Delay` 0.2)
      (`/Engine/EditorBlueprintResources/StandardMacros.IsValid` (`self.TopDownGrid`)
        (:`Is Valid`
          (`MaterialInstanceDynamic.SetScalarParameterValue` (`self.PostProcessDMI`) "GridBias" (/ 1.0 (`KismetMathLibrary.Conv_IntToDouble` (* (`TopDownGrid.GetGridVolumeExtentXY` (`self.TopDownGrid`)) 2))))
          (`KismetSystemLibrary.K2_SetTimerDelegate` (`|CreateDelegate` :!event `UpdateFogPostPorcess`) (/ 1.0 (`KismetMathLibrary.Conv_ByteToDouble` (`self.FogUpdateInterval`))) true))))))

(event `UpdateFogPostPorcess`
  (bind _asbp_top_down_player_controller (cast `/Game/TopDown/Blueprints/BP_TopDownPlayerController` (`GameplayStatics.GetPlayerController` 0)))
  (`Image.SetBrushFromTexture` (`/Game/TopDown/Blueprints/WBP_MiniMap.MinimapImage` (`/Game/TopDown/Blueprints/BP_TopDownPlayerController.MiniMapWBP` _asbp_top_down_player_controller)) (`self.FogTexture`) false)
  (`MaterialInstanceDynamic.SetTextureParameterValue` (`self.PostProcessDMI`) "FogTexture" (`self.FogTexture`)))

(fn `UserConstructionScript`)