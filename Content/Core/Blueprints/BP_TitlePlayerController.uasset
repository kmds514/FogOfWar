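; BP_TitlePlayerController is the player controller for the title screen, handling the title menu and multiplayer session entry.
; On BeginPlay it switches to UI-only input and, for the local controller, creates the WBP_Title widget if needed and adds it to the viewport.
; StartServer opens the Lobby map as a listen server, and ConnectServer joins a host by opening the given IP address as a level.
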(event `self.ReceiveBeginPlay`
  (`|ExecutionSequence`
    (:`then_0`
      (`WidgetBlueprintLibrary.SetInputMode_UIOnlyEx` self null))
    (:`then_1`
      (if (`self.IsLocalPlayerController`)
        (`/Engine/EditorBlueprintResources/StandardMacros.IsValid` (`self.TitleWBP`)
          (:`Is Valid`
            _)
          (:`Is Not Valid`
            (bind _returnvalue (`|CreateWidget` "/Game/UI/Blueprints/WBP_Title.WBP_Title_C" self))
            (set `self.TitleWBP` _returnvalue)))
        (`UserWidget.AddToViewport` (`self.TitleWBP`) 0)))))

(fn `ConnectServer`
  (params (IPAddress :type "String (by ref)"))
  (`GameplayStatics.OpenLevel` (`KismetStringLibrary.Conv_StringToName` IPAddress)))

(fn `StartServer`
  (`GameplayStatics.OpenLevel` "Lobby" true "listen"))

(fn `UserConstructionScript`)