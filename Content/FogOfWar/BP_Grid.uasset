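; Grid actor for fog of war that maps world locations to square tile coordinates and back within a box volume.
; Construction sizes the volume from GridExtent and derives a transform scaled to one tile, so conversions are transform operations with a half-grid shift.
; Coordinate-to-world snaps tile centers to surfaces by tracing downward, falling back to a second channel on a miss.
; Optional debug draws persistent tile boxes and trace lines.
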(fn `DrawDebug`
  (locals (X :type Integer) (Y :type Integer) (Location :type "Vector Structure"))
  (bind _returnvalue (- (`self.GridUnit`) 1))
  (if (or (`self.DebugGrid`) (`self.DebugLine`))
    (for _index (range (+ _returnvalue 1))
      (set `local.X` _index)
      (for _index_2 (range (+ _returnvalue 1))
        (set `local.Y` _index_2)
        (`KismetSystemLibrary.DrawDebugBox` (`self.TransformCoordsToWorld` (make `IntPoint` (`local.X`) (`local.Y`))) (`self.TileExtent`) (struct :`G` 0.2 :`A` 1.0) (struct) 3600.0 5.0)))))

(fn `LineTraceByMinusZAxis`
  (params (Start :type "Vector Structure (by ref)"))
  (returns (`Hit Impact Point` :type "Vector Structure"))
  (locals (TraceBegin :type "Vector Structure") (TraceEnd :type "Vector Structure"))
  (bind (_gridextent_x _gridextent_y _gridextent_z) (`KismetMathLibrary.BreakVector` (`self.GridExtent`)))
  (bind _returnvalue (select `bool` (`self.DebugLine`) :`true` "Persistent" :!type "EDrawDebugTrace Enum"))
  (bind _output_get (set `local.TraceBegin` Start))
  (set `local.TraceEnd` (`KismetMathLibrary.MakeVector` (.x _output_get) (.y _output_get) (- (.z _output_get) (* 2 _gridextent_z))))
  (bind _outhit (`KismetSystemLibrary.LineTraceSingle` :`Start` (`local.TraceBegin`) :`End` (`local.TraceEnd`) :`TraceChannel` "TraceTypeQuery4" :`DrawDebugType` _returnvalue))
  (if (`GameplayStatics.BreakHitResult` _outhit)
    (return (`.ImpactPoint` (`GameplayStatics.BreakHitResult` _outhit)))
    (else
      (bind _outhit_2 (`KismetSystemLibrary.LineTraceSingle` :`Start` (`local.TraceBegin`) :`End` (`local.TraceEnd`) :`TraceChannel` "TraceTypeQuery3" :`DrawDebugType` _returnvalue))
      (if (`GameplayStatics.BreakHitResult` _outhit_2)
        (return (`.ImpactPoint` (`GameplayStatics.BreakHitResult` _outhit_2)))))))

(fn `TransformCoordsToWorld`
  (params (Coords :type "IntPoint Structure"))
  (returns (WorldLocation :type "Vector Structure"))
  (locals (Location :type "Vector Structure"))
  (bind (_gridextent_x _gridextent_y _gridextent_z) (`KismetMathLibrary.BreakVector` (`self.GridExtent`)))
  (bind _output_get (set `local.Location` (`KismetMathLibrary.MakeVector` (`KismetMathLibrary.Conv_IntToDouble` (- Coords_X (`self.Shift`))) (`KismetMathLibrary.Conv_IntToDouble` (- Coords_Y (`self.Shift`))))))
  (return (`self.LineTraceByMinusZAxis` (+ (+ (`KismetMathLibrary.TransformLocation` (`self.VolumeTransform`) _output_get) (`self.TileExtent`)) (`KismetMathLibrary.MakeVector` 0.0 0.0 _gridextent_z)))))

(fn `TransformWorldToCoords`
  (params (WorldLocation :type "Vector Structure (by ref)"))
  (returns (Coords :type "IntPoint Structure"))
  (bind (_returnvalue_x _returnvalue_y) (`KismetMathLibrary.BreakVector` (`KismetMathLibrary.InverseTransformLocation` (`self.VolumeTransform`) WorldLocation)))
  (bind _returnvalue (- (`self.GridUnit`) 1))
  (return (make `IntPoint` (`KismetMathLibrary.Clamp` (+ (`self.Shift`) (`KismetMathLibrary.FFloor` _returnvalue_x)) 0 _returnvalue) (`KismetMathLibrary.Clamp` (+ (`self.Shift`) (`KismetMathLibrary.FFloor` _returnvalue_y)) 0 _returnvalue))))

(fn `UpdateVolumeTranform`
  (bind _volume (`self.Volume`))
  (bind (_returnvalue_x _returnvalue_y) (`KismetMathLibrary.BreakVector` (/ (`.BoxExtent` (`KismetSystemLibrary.GetComponentBounds` (`self.Volume`))) (`self.GridUnit`))))
  (set `self.Shift` (/ (`self.GridUnit`) 2))
  (set `self.VolumeTransform` (`KismetMathLibrary.MakeTransform` (`SceneComponent.K2_GetComponentLocation` _volume) (`SceneComponent.K2_GetComponentRotation` _volume) (/ (* (`.BoxExtent` (`KismetSystemLibrary.GetComponentBounds` _volume)) 2.0) (`KismetMathLibrary.Conv_IntToDouble` (`self.GridUnit`)))))
  (set `self.TileExtent` (`KismetMathLibrary.MakeVector` _returnvalue_x _returnvalue_y)))

(fn `UserConstructionScript`
  (`|ExecutionSequence`
    (:`then_0`
      (`KismetSystemLibrary.FlushPersistentDebugLines`))
    (:`then_1`
      (`BoxComponent.SetBoxExtent` (`self.Volume`) (`self.GridExtent`) true))
    (:`then_3`
      (`self.UpdateVolumeTranform`)
      (`self.DrawDebug`))))