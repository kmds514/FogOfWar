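; Lobby game mode that registers joining players, syncs lobby state to clients and starts the match.
; On PostLogin it reads lobby settings from the game instance, assigns each lobby controller a free player slot and creates its menu via client calls.
; Server events rebuild the player list and store map selection, pushing both to all controllers.
; StartGame runs a servertravel console command to the map selected by MapId.
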(event `self.K2_PostLogin`
  (params (NewPlayer :type "PlayerController Object Reference"))
  ;[1 0 0] OnPostLogin
  (`/Engine/EditorBlueprintResources/ActorMacros.Switch Has Authority`
    (:`Authority`
      (`|ExecutionSequence`
        (:`then_0`
          (`KismetArrayLibrary.Array_Add` (`self.AllPlayerControllers`) NewPlayer)
          (bind _asbp_game_instance (cast `/Game/Core/Blueprints/BP_GameInstance` (`GameplayStatics.GetGameInstance`)))
          (set `self.LobbyName` (`/Game/Core/Blueprints/BP_GameInstance.LobbyName` _asbp_game_instance))
          (set `self.MaxPlayers` (`/Game/Core/Blueprints/BP_GameInstance.MaxPlayers` _asbp_game_instance)))
        (:`then_1`
          ;[1 1 1] 플레이어 컨트롤러 초기화
          (bind _asbp_lobby_player_controller (cast `/Game/Core/Blueprints/BP_LobbyPlayerController` NewPlayer))
          (`|ExecutionSequence`
            (:`then_0`
              (for (_array_element _array_index) (`self.AvailablePlayerIndex`)
                (if (== _array_element true)
                  (`|VariableSetRef` (`|GetArrayItem` (`self.AvailablePlayerIndex`) _array_index))
                  (`/Game/Core/Blueprints/BP_LobbyPlayerController.Client_InitializeLobbyPC` _asbp_lobby_player_controller _array_index)
                  (break))))
            (:`then_1`
              ;[1 1 1] LobbyMenu 위젯 생성
              (`/Game/Core/Blueprints/BP_LobbyPlayerController.Client_CreateLobbyMenu` _asbp_lobby_player_controller (`self.LobbyName`))
              (`/Game/Core/Blueprints/BP_LobbyPlayerController.Client_UpdateLobbySettings` _asbp_lobby_player_controller (`self.MapImage`) (`self.MapName`)))))
        (:`then_2`
          ;[1 1 1] 다른 플레이어들에게 로비 정보를 업데이트하라고 알림
          (`self.Server_UpdatePlayerInfo`))))))

(event `Server_UpdatePlayerInfo`
  (bind _allplayercontrollers (`self.AllPlayerControllers`))
  ;[1 1 1] 클라이언트에게 PlayerInfo를 업데이트하라고 호출
  (bind _output_get (set `self.CurrentPlayers` (`KismetArrayLibrary.Array_Length` (`self.AllPlayerControllers`))))
  (if (> _output_get 0)
    (`KismetArrayLibrary.Array_Clear` (`self.ConnectedPlayersInfo`))
    (for _array_element _allplayercontrollers
      (bind _asbp_lobby_player_controller (cast `/Game/Core/Blueprints/BP_LobbyPlayerController` _array_element))
      (`KismetArrayLibrary.Array_Add` (`self.ConnectedPlayersInfo`) (`/Game/Core/Blueprints/BP_LobbyPlayerController.PlayerInfo` _asbp_lobby_player_controller)))
    (for _array_element_2 _allplayercontrollers
      (bind _asbp_lobby_player_controller_2 (cast `/Game/Core/Blueprints/BP_LobbyPlayerController` _array_element_2))
      (`/Game/Core/Blueprints/BP_LobbyPlayerController.Client_AddPlayerInfo` _asbp_lobby_player_controller_2 (`self.ConnectedPlayersInfo`)))))

(event `Server_UpdateGameSettings`
  (params (MapImage :type "Texture2D Object Reference") (MapName :type Text) (MapId :type Integer))
  ;[1 1 1] 클라이언트에게 로비 정보를 업데이트하라고 호출
  (set `self.MapImage` MapImage)
  (set `self.MapName` MapName)
  (set `self.MapId` MapId)
  (for _array_element (`self.AllPlayerControllers`)
    (bind _asbp_lobby_player_controller (cast `/Game/Core/Blueprints/BP_LobbyPlayerController` _array_element))
    (`/Game/Core/Blueprints/BP_LobbyPlayerController.Client_UpdateLobbySettings` _asbp_lobby_player_controller (`self.MapImage`) (`self.MapName`))))

(event `StartGame`
  ;[1 1 1] 로비에서 선택한 맵으로 게임 시작
  (`KismetSystemLibrary.ExecuteConsoleCommand` (select `int` (`self.MapId`) :`0` "servertravel /Game/Core/Maps/TopDownExampleMap" :`1` "servertravel /Game/Core/Maps/DreamscapeMeadows" :`2` "servertravel /Game/Core/Maps/LostRuin") (`GameplayStatics.GetPlayerController` 0)))

(fn `UserConstructionScript`)