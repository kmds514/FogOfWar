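; Grid actor that builds the terrain tile map and drives its fog of war.
; Construction traces down through a box volume to store each tile's location and BP_Terrain height; BeginPlay spawns BP_Tile actors from that data.
; A looping timer paints fog states into a render target, one pixel per tile, then demotes revealed tiles to grey.
; Tick alpha-blends that target into a second one for smooth fades; helpers provide index conversion and area queries.
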(event `self.ReceiveBeginPlay`
  (`|ExecutionSequence`
    (:`then_0`
      ;[1 1 1] Spawns Tiles
      (bind _keys (`BlueprintMapLibrary.Map_Keys` (`self.TileData`)))
      (for _array_element _keys
        (bind _value (`BlueprintMapLibrary.Map_Find` (`self.TileData`) _array_element))
        (bind _returnvalue (`|SpawnActorFromClass` "/Game/Grid/BP_Tile.BP_Tile_C" (`KismetMathLibrary.Conv_VectorToTransform` (break `/Game/Grid/FTile` _value)) "Undefined" "OverrideRootScale" null self (`self.TileExtent`) (`.GridIndex_10_F4FE481C465A80AA605C6CBD57E37F72` (break `/Game/Grid/FTile` _value)) (`.Height_2_E06127354CF358B3104C56AE0FB087BD` (break `/Game/Grid/FTile` _value)) (`.FogState_16_AA550FFF4E17253B98CF1287A859FD25` (break `/Game/Grid/FTile` _value)) (`self.ShowDebugTile`) null))
        (`BlueprintMapLibrary.Map_Add` (`self.Tiles`) (`.GridIndex_10_F4FE481C465A80AA605C6CBD57E37F72` (break `/Game/Grid/FTile` _value)) _returnvalue)))
    (:`then_1`
      (`KismetRenderingLibrary.ClearRenderTarget2D` (`self.FogOfWarCanvasRT`))
      (`KismetRenderingLibrary.ClearRenderTarget2D` (`self.FogOfWarInterpCanvasRT`))
      (`KismetSystemLibrary.K2_SetTimer` null "OnFogChange" 0.1 true))))

(event `self.ReceiveTick`
  (params (DeltaSeconds :type "Float (single-precision)"))
  (`|ExecutionSequence`
    (:`then_0`
      (bind (_canvas _size _context) (`KismetRenderingLibrary.BeginDrawCanvasToRenderTarget` (`self.FogOfWarInterpCanvasRT`)))
      (`Canvas.K2_DrawTexture` _canvas (`self.FogOfWarCanvasRT`) (0.0 0.0) _size (0.0 0.0) (1.0 1.0) (`KismetMathLibrary.MakeColor` 1.0 1.0 1.0 (* (`GameplayStatics.GetWorldDeltaSeconds`) 3.0)) "BLEND_Translucent" 0.0 (0.5 0.5))
      (`KismetRenderingLibrary.EndDrawCanvasToRenderTarget` _context))))

(fn `DrawDebugTile`
  (if (`self.ShowDebugTile`)
    (bind _keys (`BlueprintMapLibrary.Map_Keys` (`self.TileData`)))
    (for _array_element _keys
      (bind (_worldlocation _gridindex _height) (break `/Game/Grid/FTile` (`BlueprintMapLibrary.Map_Find` (`self.TileData`) _array_element)))
      (bind _returnvalue (+ (.z _worldlocation) 1.0))
      (`KismetSystemLibrary.DrawDebugPlane` (`KismetMathLibrary.MakePlaneFromPointAndNormal` (`KismetMathLibrary.MakeVector` (.x _worldlocation) (.y _worldlocation) _returnvalue) (0.0 0.0 1.0)) (`KismetMathLibrary.MakeVector` (.x _worldlocation) (.y _worldlocation) _returnvalue) (* (`self.TileExtent`) 0.9) (select `/Game/Grid/ETileHeight` _height :`NewEnumerator0` (struct :`R` 0.01 :`G` 0.01 :`B` 0.01 :`A` 1.0) :`NewEnumerator1` (struct :`R` 0.1 :`G` 0.4 :`A` 1.0) :`NewEnumerator2` (struct :`R` 0.2 :`G` 0.3 :`A` 1.0) :`NewEnumerator3` (struct :`R` 0.3 :`G` 0.2 :`A` 1.0) :`NewEnumerator4` (struct :`R` 0.4 :`G` 0.1 :`A` 1.0) :!type "LinearColor Structure") 36000.0)))
  (return))

(fn `GenerateTileData`
  (locals (X :type Integer) (Y :type Integer))
  (bind (_numx _numy) (`self.GetNumOfTiles`))
  (bind _x (`local.X`))
  (bind _y (`local.Y`))
  (bind (_hit_impact_point _height) (`self.LineTraceByMinusZAxis` (+ (`self.GetOrigin`) (* (`self.GetActorForwardVector`) (+ (* (`local.X`) (* 2 (`self.TileExtent`))) (`self.TileExtent`))) (* (`self.GetActorRightVector`) (+ (* (`local.Y`) (* 2 (`self.TileExtent`))) (`self.TileExtent`))))))
  (for _index (range (+ _numx 1))
    (set `local.X` _index)
    (for _index_2 (range (+ _numy 1))
      (set `local.Y` _index_2)
      (`BlueprintMapLibrary.Map_Add` (`self.TileData`) (make `IntPoint` _x _y) (make `/Game/Grid/FTile` _hit_impact_point (make `IntPoint` _x _y) _height)))))

(fn `GetDistToRadius`
  (params (Center :type "/Game/Grid/FTile Structure (by ref)") (Radius :type Integer))
  (returns (Distance :type "Float (double-precision)"))
  (bind (_worldlocation _gridindex) (break `/Game/Grid/FTile` (`local.Center`)))
  (return (`KismetMathLibrary.FMax` (`KismetMathLibrary.Vector_Distance2DSquared` _worldlocation (break `/Game/Grid/FTile` (`BlueprintMapLibrary.Map_Find` (`self.TileData`) (make `IntPoint` (+ (`local.Radius`) (break `IntPoint` _gridindex)) (`.Y` (break `IntPoint` _gridindex)))))) (`KismetMathLibrary.Vector_Distance2DSquared` _worldlocation (break `/Game/Grid/FTile` (`BlueprintMapLibrary.Map_Find` (`self.TileData`) (make `IntPoint` (break `IntPoint` _gridindex) (+ (`local.Radius`) (`.Y` (break `IntPoint` _gridindex))))))) (`KismetMathLibrary.Vector_Distance2DSquared` _worldlocation (break `/Game/Grid/FTile` (`BlueprintMapLibrary.Map_Find` (`self.TileData`) (make `IntPoint` (- (`local.Radius`) (break `IntPoint` _gridindex)) (`.Y` (break `IntPoint` _gridindex)))))) (`KismetMathLibrary.Vector_Distance2DSquared` _worldlocation (break `/Game/Grid/FTile` (`BlueprintMapLibrary.Map_Find` (`self.TileData`) (make `IntPoint` (break `IntPoint` _gridindex) (- (`local.Radius`) (`.Y` (break `IntPoint` _gridindex))))))))))

(fn `GetNumOfTiles`
  (returns (NumX :type Integer) (NumY :type Integer))
  (bind (_gridextent_x _gridextent_y) (`KismetMathLibrary.BreakVector` (`self.GridExtent`)))
  (bind _tileextent (`self.TileExtent`))
  (return (- (`KismetMathLibrary.FFloor` (/ _gridextent_x _tileextent)) 1) (- (`KismetMathLibrary.FFloor` (/ _gridextent_y _tileextent)) 1)))

(fn `GetOrigin`
  (returns (Location :type "Vector Structure"))
  (return (`KismetMathLibrary.MakeVector` (- (.x (`self.GridLocation`)) (.x (`self.GridExtent`))) (- (.y (`self.GridLocation`)) (.y (`self.GridExtent`))) (+ (.z (`self.GridLocation`)) (.z (`self.GridExtent`))))))

(fn `GetRectArea`
  (params (Center :type "/Game/Grid/FTile Structure (by ref)") (Radius :type Integer))
  (returns (RectArea :type "Array of /Game/Grid/FTile Structure"))
  (locals (Rect :type "Array of /Game/Grid/FTile Structure") (X :type Integer) (Y :type Integer))
  (bind _radius (`local.Radius`))
  (bind _radius_2 (`local.Radius`))
  (bind (_worldlocation _gridindex) (break `/Game/Grid/FTile` (`local.Center`)))
  (bind (_worldlocation_2 _gridindex_2) (break `/Game/Grid/FTile` (`local.Center`)))
  (bind (_value _returnvalue) (`BlueprintMapLibrary.Map_Find` (`self.TileData`) (make `IntPoint` (`local.X`) (`local.Y`))))
  (for _index (range (- (break `IntPoint` _gridindex_2) _radius_2) (+ (+ (break `IntPoint` _gridindex_2) _radius_2) 1))
    (set `local.X` _index)
    (for _index_2 (range (- (`.Y` (break `IntPoint` _gridindex)) _radius) (+ (+ (`.Y` (break `IntPoint` _gridindex)) _radius) 1))
      (set `local.Y` _index_2)
      (if _returnvalue
        (`KismetArrayLibrary.Array_Add` (`local.Rect`) _value))))
  (return (`local.Rect`)))

(fn `IndexToLocation`
  (params (GridIndex :type "IntPoint Structure (by ref)"))
  (returns (WorldLocation :type "Vector Structure"))
  (return (break `/Game/Grid/FTile` (`BlueprintMapLibrary.Map_Find` (`self.TileData`) GridIndex))))

(fn `LineTraceByMinusZAxis`
  (params (Start :type "Vector Structure (by ref)"))
  (returns (`Hit Impact Point` :type "Vector Structure") (Height :type "/Game/Grid/ETileHeight Enum"))
  (locals (TraceBegin :type "Vector Structure") (TraceEnd :type "Vector Structure"))
  (bind (_gridextent_x _gridextent_y _gridextent_z) (`KismetMathLibrary.BreakVector` (`self.GridExtent`)))
  (bind _returnvalue (select `bool` (`self.ShowDebugTraceLine`) :`true` "Persistent" :!type "EDrawDebugTrace Enum"))
  (bind _output_get (set `local.TraceBegin` Start))
  (set `local.TraceEnd` (`KismetMathLibrary.MakeVector` (.x _output_get) (.y _output_get) (- (.z _output_get) (* 2 _gridextent_z))))
  (bind _outhit (`KismetSystemLibrary.LineTraceSingle` :`Start` (`local.TraceBegin`) :`End` (`local.TraceEnd`) :`TraceChannel` "TraceTypeQuery4" :`DrawDebugType` _returnvalue))
  (if (`GameplayStatics.BreakHitResult` _outhit)
    (return (`.ImpactPoint` (`GameplayStatics.BreakHitResult` _outhit)) (`/Game/Grid/BP_Terrain.Height` (cast `/Game/Grid/BP_Terrain` (`.HitActor` (`GameplayStatics.BreakHitResult` _outhit)) :!pure true)))
    (else
      (bind _outhit_2 (`KismetSystemLibrary.LineTraceSingle` :`Start` (`local.TraceBegin`) :`End` (`local.TraceEnd`) :`TraceChannel` "TraceTypeQuery3" :`DrawDebugType` _returnvalue))
      (if (`GameplayStatics.BreakHitResult` _outhit_2)
        (return (`.ImpactPoint` (`GameplayStatics.BreakHitResult` _outhit_2)) (`/Game/Grid/BP_Terrain.Height` (cast `/Game/Grid/BP_Terrain` (`.HitActor` (`GameplayStatics.BreakHitResult` _outhit_2)) :!pure true)))))))

(fn `LocationToIndex`
  (params (WorldLocation :type "Vector Structure (by ref)"))
  (returns (GridIndex :type "IntPoint Structure"))
  (bind (_returnvalue_x _returnvalue_y) (`KismetMathLibrary.BreakVector` (- WorldLocation (`self.GetOrigin`))))
  (bind _returnvalue (* 2 (`self.TileExtent`)))
  (return (make `IntPoint` (`.ReturnValue` (`KismetMathLibrary.FMod` _returnvalue_x _returnvalue)) (`.ReturnValue` (`KismetMathLibrary.FMod` _returnvalue_y _returnvalue)))))

(fn `OnFogChange`
  (locals (Canvas :type "Canvas Object Reference") (Tile :type "/Game/Grid/BP_Tile Object Reference"))
  (bind (_canvas _size _context) (`KismetRenderingLibrary.BeginDrawCanvasToRenderTarget` (`self.FogOfWarCanvasRT`)))
  (set `local.Canvas` _canvas)
  (`Canvas.K2_DrawTexture` (`local.Canvas`) null (0.0 0.0) _size (0.0 0.0) (1.0 1.0) (struct :`A` 1.0) "BLEND_Opaque" 0.0 (0.5 0.5))
  (bind _keys (`BlueprintMapLibrary.Map_Keys` (`self.Tiles`)))
  (for _array_element _keys
    (set `local.Tile` (`BlueprintMapLibrary.Map_Find` (`self.Tiles`) _array_element))
    (`Canvas.K2_DrawTexture` (`local.Canvas`) null (`KismetMathLibrary.Conv_IntPointToVector2D` (`/Game/Grid/BP_Tile.GridIndex` (`local.Tile`))) (1.0 1.0) (0.0 0.0) (1.0 1.0) (select `/Game/Grid/EFogState` (`/Game/Grid/BP_Tile.FogState` (`local.Tile`)) :`NewEnumerator2` (struct :`R` 0.1 :`G` 0.1 :`B` 0.1 :`A` 1.0) :`NewEnumerator3` (struct :`R` 1.0 :`G` 1.0 :`B` 1.0 :`A` 1.0) :!type "LinearColor Structure") "BLEND_Translucent" 0.0 (0.5 0.5))
    (if (`|EnumEquality` (`/Game/Grid/BP_Tile.FogState` (`local.Tile`)) "NewEnumerator3")
      (`/Game/Grid/BP_Tile.ToGrey` (`local.Tile`))))
  (`KismetRenderingLibrary.EndDrawCanvasToRenderTarget` _context))

(fn `UserConstructionScript`
  (if (`self.Refresh`)
    _
    (else
      _))
  (`|ExecutionSequence`
    (:`then_0`
      (`self.K2_SetActorRotation` (`self.LockRotation`))
      (`KismetSystemLibrary.FlushPersistentDebugLines`))
    (:`then_1`
      (set `self.GridLocation` (`SceneComponent.K2_GetComponentLocation` (`self.GridVolume`)))
      (`BoxComponent.SetBoxExtent` (`self.GridVolume`) (`self.GridExtent`) true)
      (`KismetSystemLibrary.DrawDebugBox` (`self.GetOrigin`) (15.0 15.0 15.0) (struct :`R` 1.0 :`A` 1.0) (struct) 36000.0 3.0) ; Draw grid origin
    )
    (:`then_2`
      (`self.GenerateTileData`))
    (:`then_4`
      (set `self.Refresh` false))))